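; BP_Turret2 is a turret that tracks and shoots at the player while they are inside its Collision volume.
; Each Tick, unless stunned, it interpolates BarrelHead toward the player's Mesh2P with a fixed DeltaTime, making rotation frame-rate dependent.
; It spawns BP_TurretProjectile at ProjectileSpawn, throttled by a game-time timestamp and ShootDelay.
; A FirstPersonProjectile overlapping Box stuns it temporarily through a delayed reset.
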(event OnComponentBeginOverlap(Collision)
  (params (OverlappedComponent :type Primitive%20Component%20Object%20Reference) (OtherActor :type Actor%20Object%20Reference) (OtherComp :type Primitive%20Component%20Object%20Reference) (OtherBodyIndex :type Integer) (bFromSweep :type Boolean) (SweepResult :type Hit%20Result%20Structure%20%28by%20ref%29))
  (if (not (Variables|Default|GetPlayerFound))
    (bind _asbp_character (Utilities|Casting|CastToBP_Character OtherActor))
    (Variables|Default|SetPlayerFound true)))

(event OnComponentEndOverlap(Collision)
  (params (OverlappedComponent :type Primitive%20Component%20Object%20Reference) (OtherActor :type Actor%20Object%20Reference) (OtherComp :type Primitive%20Component%20Object%20Reference) (OtherBodyIndex :type Integer))
  (Utilities|Casting|CastToBP_Character OtherActor)
  (Variables|Default|SetPlayerFound false))

(event OnComponentBeginOverlap(Box)
  (params (OverlappedComponent :type Primitive%20Component%20Object%20Reference) (OtherActor :type Actor%20Object%20Reference) (OtherComp :type Primitive%20Component%20Object%20Reference) (OtherBodyIndex :type Integer) (bFromSweep :type Boolean) (SweepResult :type Hit%20Result%20Structure%20%28by%20ref%29))
  (Utilities|Casting|CastToFirstPersonProjectile OtherActor)
  (Variables|Default|Setstunned true)
  (CallFunction|StunTIMER))

(event Custom|Shoot%20Player
  (bind _barrelhead (Variables|Default|GetBarrelHead))
  (if (not (Variables|Default|Getstunned))
    (if (Variables|Default|GetPlayerFound)
      (Transformation|SetWorldRotation (Variables|Default|GetBarrelHead) (Math|Interpolation|RInterpTo (Transformation|GetWorldRotation _barrelhead) (Math|Rotator|FindLookatRotation (Transformation|GetWorldLocation _barrelhead) (Transformation|GetWorldLocation (Variables|/Game/Ninja/BP_Character.BP_Character_C|GetMesh2P (stale OnComponentBeginOverlap(Collision) _asbp_character)))) 1.0 (Variables|Default|GetTurretRotationSpeed)) false false)
      (CallFunction|SpawnProjectile))))

(event Custom|Stun%20tImer
  (Utilities|FlowControl|Delay 5.0)
  (Variables|Default|Setstunned false))

(event EventTick
  (params (DeltaSeconds :type Float%20%28single-precision%29))
  (CallFunction|ShootPlayer))

(fn ConstructionScript)

(fn SpawnProjectile
  (bind _returnvalue (Utilities|Time|GetGameTimeinSeconds))
  (if (> _returnvalue (Variables|Default|GetGameTimeShoot))
    (Variables|Default|SetGameTimeShoot (+ _returnvalue (Variables|Default|GetShootDelay)))
    (Game|SpawnActorfromClass "/Game/Ninja/BP_TurretProjectile.BP_TurretProjectile_C" (Transformation|GetWorldTransform (Variables|Default|GetProjectileSpawn)) "Undefined" 0 0)))