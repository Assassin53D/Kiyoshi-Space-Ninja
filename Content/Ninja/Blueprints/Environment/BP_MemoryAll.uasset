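; BP_MemoryAll is a trigger volume that unlocks a player ability: wall climb, dash or deflect.
; When BP_Character overlaps its Box, the first true flag in that order enables the matching ability and reveals its PlayerWidget UI through GameUIRef.
; Wall climb also plays a W_Cutscene, guarded by WallPlayed to run once per actor.
; Similar cutscene calls, presumably for dash and deflect, are disconnected and never run.
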(event OnComponentBeginOverlap(Box)
  (params (OverlappedComponent :type Primitive%20Component%20Object%20Reference) (OtherActor :type Actor%20Object%20Reference) (OtherComp :type Primitive%20Component%20Object%20Reference) (OtherBodyIndex :type Integer) (bFromSweep :type Boolean) (SweepResult :type Hit%20Result%20Structure%20%28by%20ref%29))
  (bind _asbp_character (Utilities|Casting|CastToBP_Character OtherActor))
  (if (Variables|Default|GetWallClimb)
    (Variables|/Game/Ninja/Blueprints/Character/BP_Character.BP_Character_C|SetCanWallClimb _asbp_character true)
    (bind _asplayer_widget (Utilities|Casting|CastToPlayerWidget (Variables|/Game/Ninja/Blueprints/Character/BP_Character.BP_Character_C|GetGameUIRef _asbp_character)))
    (Widget|SetVisibility (Variables|/Game/Ninja/UI/PlayerWidget.PlayerWidget_C|GetGripBar _asplayer_widget) "Visible")
    (if (not (Variables|Default|GetwallPlayed))
      (Variables|Default|SetwallPlayed true)
      (bind _returnvalue (UserInterface|CreateWidget "/Game/Ninja/Cutscenes/W_Cutscene.W_Cutscene_C"))
      (UserInterface|Viewport|AddtoViewport _returnvalue 0)
      (Default|PlayCutscene _returnvalue 2))
    (elif (Variables|Default|GetDash)
      (Variables|/Game/Ninja/Blueprints/Character/BP_Character.BP_Character_C|SetCanDash _asbp_character true)
      (bind _asplayer_widget_2 (Utilities|Casting|CastToPlayerWidget (Variables|/Game/Ninja/Blueprints/Character/BP_Character.BP_Character_C|GetGameUIRef _asbp_character)))
      (Widget|SetVisibility (Variables|/Game/Ninja/UI/PlayerWidget.PlayerWidget_C|GetDashBar _asplayer_widget_2) "Visible")
      (elif (Variables|Default|GetDeflect)
        (Variables|/Game/Ninja/Blueprints/Character/BP_Character.BP_Character_C|SetCanDeflect _asbp_character true)
        (bind _asplayer_widget_3 (Utilities|Casting|CastToPlayerWidget (Variables|/Game/Ninja/Blueprints/Character/BP_Character.BP_Character_C|GetGameUIRef _asbp_character)))
        (Widget|SetVisibility (Variables|/Game/Ninja/UI/PlayerWidget.PlayerWidget_C|GetDeflectBar _asplayer_widget_3) "Visible")))))

(event EventBeginPlay)

(event Collision|EventActorBeginOverlap
  (params (OtherActor :type Actor%20Object%20Reference)))

(event EventTick
  (params (DeltaSeconds :type Float%20%28single-precision%29)))

(fn ConstructionScript)