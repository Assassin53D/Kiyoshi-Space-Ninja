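; Switch actor that sets an IsActive flag when a BP_Interaction actor overlaps its interaction volume or a FirstPersonProjectile overlaps its box.
; Activation is ignored while HasNoPower is set.
; A point light shows green when ready and red when activated or unpowered, with the initial color chosen on BeginPlay.
; When CanBeReused is set, TurnOff clears the flag and restores green after a short delay.
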(event OnComponentBeginOverlap(InteractionCollision)
  (params (OverlappedComponent :type Primitive%20Component%20Object%20Reference) (OtherActor :type Actor%20Object%20Reference) (OtherComp :type Primitive%20Component%20Object%20Reference) (OtherBodyIndex :type Integer) (bFromSweep :type Boolean) (SweepResult :type Hit%20Result%20Structure%20%28by%20ref%29))
  (Utilities|Casting|CastToBP_Interaction OtherActor)
  (if (not (Variables|Default|GetHasNoPower))
    (Variables|Default|SetIsActive true)
    (Rendering|Components|Light|SetLightColor (Variables|Default|GetPointLight) "(R=1.000000,G=0.000000,B=0.000000,A=1.000000)" true)
    (if (Variables|Default|GetCanBeReused)
      (CallFunction|TurnOff))))

(event OnComponentBeginOverlap(Box)
  (params (OverlappedComponent :type Primitive%20Component%20Object%20Reference) (OtherActor :type Actor%20Object%20Reference) (OtherComp :type Primitive%20Component%20Object%20Reference) (OtherBodyIndex :type Integer) (bFromSweep :type Boolean) (SweepResult :type Hit%20Result%20Structure%20%28by%20ref%29))
  (Utilities|Casting|CastToFirstPersonProjectile OtherActor)
  (if (not (Variables|Default|GetHasNoPower))
    (Variables|Default|SetIsActive true)
    (Development|PrintString "Hello")
    (Rendering|Components|Light|SetLightColor (Variables|Default|GetPointLight) "(R=1.000000,G=0.000000,B=0.000000,A=1.000000)" true)
    (if (Variables|Default|GetCanBeReused)
      (CallFunction|TurnOff))))

(event Custom|TurnOff
  (Utilities|FlowControl|Delay 3.0)
  (Variables|Default|SetIsActive false)
  (Rendering|Components|Light|SetLightColor (Variables|Default|GetPointLight) "(R=0.000000,G=1.000000,B=0.130136,A=1.000000)" true))

(event Custom|Power
  (bind _pointlight (Variables|Default|GetPointLight))
  (if (Variables|Default|GetHasNoPower)
    (Rendering|Components|Light|SetLightColor _pointlight "(R=1.000000,G=0.000000,B=0.000000,A=1.000000)" true)
    (else
      (Rendering|Components|Light|SetLightColor _pointlight "(R=0.100000,G=1.000000,B=0.000000,A=1.000000)" true))))

(event EventBeginPlay
  (CallFunction|Power))

(event Collision|EventActorBeginOverlap
  (params (OtherActor :type Actor%20Object%20Reference)))

(event EventTick
  (params (DeltaSeconds :type Float%20%28single-precision%29)))

(fn ConstructionScript)