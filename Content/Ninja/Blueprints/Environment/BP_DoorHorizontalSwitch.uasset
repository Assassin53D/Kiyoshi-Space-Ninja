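; Door actor that slides its static mesh upward when its LiftDoorUp event is called.
; The construction script caches the closed location and a raised target above it.
; A timeline drives the movement, feeding its track into VInterpTo as DeltaTime from the fixed closed position.
; During playback the mesh switches to a pulsing hex-tile material, and a DoOnce plays the opening sound a single time.
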(event Custom|LiftDoorUp
  (bind _staticmeshcomponent (Variables|Debug|GetStaticMeshComponent))
  (bind _newtrack_0 (Timeline|TimelineDoorUp Play)
    (:Update
      (Transformation|SetWorldLocation _staticmeshcomponent (Math|Interpolation|VInterpTo (Variables|Default|GetDoorDown) (Variables|Default|GetDoorUp) _newtrack_0 1.0) false false)
      (Rendering|Material|SetMaterial _staticmeshcomponent 0 "/Game/StarterContent/Materials/M_Tech_Hex_Tile_Pulse.M_Tech_Hex_Tile_Pulse")
      (Utilities|FlowControl|DoOnce false
        (:Completed
          (Audio|PlaySoundatLocation "/Game/Ninja/Audio/SFX_DoorOpen_01_Cue.SFX_DoorOpen_01_Cue" (Transformation|GetWorldLocation (Variables|Debug|GetStaticMeshComponent))))))))

(event EventBeginPlay)

(event Collision|EventActorBeginOverlap
  (params (OtherActor :type Actor%20Object%20Reference)))

(event EventTick
  (params (DeltaSeconds :type Float%20%28single-precision%29)))

(fn ConstructionScript
  (bind _output_get (Variables|Default|SetDoorDown (Transformation|GetWorldLocation (Variables|Debug|GetStaticMeshComponent))))
  (Variables|Default|SetDoorUp (Math|Vector|MakeVector (.X (Math|Vector|BreakVector _output_get)) (.Y (Math|Vector|BreakVector _output_get)) (+ (.Z (Math|Vector|BreakVector _output_get)) 2.5e+02))))