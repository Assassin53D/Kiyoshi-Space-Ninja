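; Vertical platform that lowers while a BP_Crates actor overlaps its Box trigger and rises back when the crate leaves.
; The construction script caches the Cube's location as the top and 500 units below it as the bottom.
; Overlap events play or reverse one timeline, whose track feeds VInterpTo's DeltaTime as a blend alpha to move the Cube.
; On finish, it records whether the platform reached the top.
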(event OnComponentBeginOverlap(Box)
  (params (OverlappedComponent :type Primitive%20Component%20Object%20Reference) (OtherActor :type Actor%20Object%20Reference) (OtherComp :type Primitive%20Component%20Object%20Reference) (OtherBodyIndex :type Integer) (bFromSweep :type Boolean) (SweepResult :type Hit%20Result%20Structure%20%28by%20ref%29))
  (Utilities|Casting|CastToBP_Crates OtherActor)
  (CallFunction|GoingDown))

(event OnComponentEndOverlap(Box)
  (params (OverlappedComponent :type Primitive%20Component%20Object%20Reference) (OtherActor :type Actor%20Object%20Reference) (OtherComp :type Primitive%20Component%20Object%20Reference) (OtherBodyIndex :type Integer))
  (Utilities|Casting|CastToBP_Crates OtherActor)
  (CallFunction|GoingUp))

(event Custom|GoingUp
  (Variables|Default|SetGoing%20Down false)
  (bind _newtrack_1 (Timeline|Timeline_0 Reverse)
    (:Update
      (Transformation|SetWorldLocation (Variables|Default|GetCube) (Math|Interpolation|VInterpTo (Variables|Default|GetDoorUp) (Variables|Default|GetDoorDown) _newtrack_1 1.0) false false))
    (:Finished
      (if (Variables|Default|GetGoing%20Down)
        (Variables|Default|SetReachedTheTop false)
        (else
          (Variables|Default|SetReachedTheTop true))))))

(event Custom|GoingDown
  (Variables|Default|SetGoing%20Down true)
  (bind _newtrack_1 (Timeline|Timeline_0 Play)
    (:Update
      (Transformation|SetWorldLocation (Variables|Default|GetCube) (Math|Interpolation|VInterpTo (Variables|Default|GetDoorUp) (Variables|Default|GetDoorDown) _newtrack_1 1.0) false false))
    (:Finished
      (if (Variables|Default|GetGoing%20Down)
        (Variables|Default|SetReachedTheTop false)
        (else
          (Variables|Default|SetReachedTheTop true))))))

(event EventBeginPlay)

(event Collision|EventActorBeginOverlap
  (params (OtherActor :type Actor%20Object%20Reference)))

(event EventTick
  (params (DeltaSeconds :type Float%20%28single-precision%29)))

(fn ConstructionScript
  (bind _output_get (Variables|Default|SetDoorUp (Transformation|GetWorldLocation (Variables|Default|GetCube))))
  (Variables|Default|SetDoorDown (Math|Vector|MakeVector (.X (Math|Vector|BreakVector _output_get)) (.Y (Math|Vector|BreakVector _output_get)) (+ (.Z (Math|Vector|BreakVector _output_get)) -5e+02))))