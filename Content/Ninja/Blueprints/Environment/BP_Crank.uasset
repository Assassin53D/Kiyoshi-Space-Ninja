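; BP_Crank is an environment crank that toggles its active state when a BP_Interaction actor or FirstPersonProjectile begins overlapping its InteractionCollision.
; Each toggle sets the Cylinder's world rotation to a positive or negative half turn, prints placeholder debug text and colors the PointLight red in both states.
; A DoOnce gates the overlap and resets only after a successful toggle, so any other overlapping actor leaves it closed.
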(event OnComponentBeginOverlap(InteractionCollision)
  (params (OverlappedComponent :type Primitive%20Component%20Object%20Reference) (OtherActor :type Actor%20Object%20Reference) (OtherComp :type Primitive%20Component%20Object%20Reference) (OtherBodyIndex :type Integer) (bFromSweep :type Boolean) (SweepResult :type Hit%20Result%20Structure%20%28by%20ref%29))
  (bind _cylinder (Variables|Default|GetCylinder))
  (Utilities|FlowControl|DoOnce false :!label _label
    (:Completed
      (Utilities|FlowControl|Sequence
        (:then_0
          (Utilities|Casting|CastToBP_Interaction OtherActor))
        (:then_1
          (Utilities|Casting|CastToFirstPersonProjectile OtherActor)))
      (if (Variables|Default|GetIsActive)
        (Variables|Default|SetIsActive false)
        (Development|PrintString "Hello")
        (Transformation|SetWorldRotation _cylinder "0, 0,180.000000" false false)
        (else
          (Variables|Default|SetIsActive true)
          (Development|PrintString "asdsa")
          (Transformation|SetWorldRotation _cylinder "0, 0,-180.000000" false false)))
      (Rendering|Components|Light|SetLightColor (Variables|Default|GetPointLight) "(R=1.000000,G=0.000000,B=0.000000,A=1.000000)" true)
      (goto _label Reset))))

(event EventBeginPlay)

(event Collision|EventActorBeginOverlap
  (params (OtherActor :type Actor%20Object%20Reference)))

(event EventTick
  (params (DeltaSeconds :type Float%20%28single-precision%29)))

(fn ConstructionScript)