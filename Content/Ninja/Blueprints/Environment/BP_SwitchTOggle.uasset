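; BP_SwitchTOggle is a switch that flips its IsActive state when triggered by an interaction or a projectile hit.
; BP_Interaction overlapping InteractionCollision, or a FirstPersonProjectile overlapping Box, drives the shared toggle logic, with the projectile destroyed on contact.
; Each toggle turns the point light blue for active or green for inactive and plays a button-press sound at the mesh.
; The DoOnce gates reset immediately, so the switch can toggle repeatedly.
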(event OnComponentBeginOverlap(InteractionCollision)
  (params (OverlappedComponent :type Primitive%20Component%20Object%20Reference) (OtherActor :type Actor%20Object%20Reference) (OtherComp :type Primitive%20Component%20Object%20Reference) (OtherBodyIndex :type Integer) (bFromSweep :type Boolean) (SweepResult :type Hit%20Result%20Structure%20%28by%20ref%29))
  (bind _staticmesh (Variables|Default|GetStaticMesh))
  (bind _pointlight (Variables|Default|GetPointLight))
  (bind _returnvalue (Transformation|GetWorldLocation _staticmesh))
  (Utilities|Casting|CastToBP_Interaction OtherActor)
  (if (Variables|Default|GetIsActive)
    (Utilities|FlowControl|DoOnce false :!label _label
      (:Completed
        (Variables|Default|SetIsActive false)
        (Rendering|Components|Light|SetLightColor _pointlight "(R=0.097587,G=1.000000,B=0.000000,A=1.000000)" true)
        (Audio|PlaySoundatLocation "/Game/Ninja/Audio/SFX_ButtonPress_01_Cue.SFX_ButtonPress_01_Cue" _returnvalue)
        (goto _label Reset)))
    (else
      (Utilities|FlowControl|DoOnce false :!label _label_2
        (:Completed
          (Variables|Default|SetIsActive true)
          (Rendering|Components|Light|SetLightColor _pointlight "(R=0.000000,G=0.295438,B=1.000000,A=1.000000)" true)
          (Audio|PlaySoundatLocation "/Game/Ninja/Audio/SFX_ButtonPress_01_Cue.SFX_ButtonPress_01_Cue" _returnvalue)
          (goto _label_2 Reset))))))

(event OnComponentBeginOverlap(Box)
  (params (OverlappedComponent :type Primitive%20Component%20Object%20Reference) (OtherActor :type Actor%20Object%20Reference) (OtherComp :type Primitive%20Component%20Object%20Reference) (OtherBodyIndex :type Integer) (bFromSweep :type Boolean) (SweepResult :type Hit%20Result%20Structure%20%28by%20ref%29))
  (bind _staticmesh (Variables|Default|GetStaticMesh))
  (bind _pointlight (Variables|Default|GetPointLight))
  (bind _returnvalue (Transformation|GetWorldLocation _staticmesh))
  (bind _asfirst_person_projectile (Utilities|Casting|CastToFirstPersonProjectile OtherActor))
  (Actor|DestroyActor _asfirst_person_projectile)
  (if (Variables|Default|GetIsActive)
    (Utilities|FlowControl|DoOnce false :!label _label
      (:Completed
        (Variables|Default|SetIsActive false)
        (Rendering|Components|Light|SetLightColor _pointlight "(R=0.097587,G=1.000000,B=0.000000,A=1.000000)" true)
        (Audio|PlaySoundatLocation "/Game/Ninja/Audio/SFX_ButtonPress_01_Cue.SFX_ButtonPress_01_Cue" _returnvalue)
        (goto _label Reset)))
    (else
      (Utilities|FlowControl|DoOnce false :!label _label_2
        (:Completed
          (Variables|Default|SetIsActive true)
          (Rendering|Components|Light|SetLightColor _pointlight "(R=0.000000,G=0.295438,B=1.000000,A=1.000000)" true)
          (Audio|PlaySoundatLocation "/Game/Ninja/Audio/SFX_ButtonPress_01_Cue.SFX_ButtonPress_01_Cue" _returnvalue)
          (goto _label_2 Reset))))))

(event EventBeginPlay)

(event Collision|EventActorBeginOverlap
  (params (OtherActor :type Actor%20Object%20Reference)))

(event EventTick
  (params (DeltaSeconds :type Float%20%28single-precision%29)))

(fn ConstructionScript)