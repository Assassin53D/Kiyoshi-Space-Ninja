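; BP_FloatingText is an environment actor that displays two configurable text lines alongside a spotlight.
; On BeginPlay it applies both strings and sets the visibility of the texts and light from the IsActive flag.
; When Rotatable is set, it turns the whole actor every Tick to face the player's BP_Character using a look-at rotation.
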(event Custom|FollowCharacter
  (if (Variables|Default|GetRotatable)
    (bind _asbp_character (Utilities|Casting|CastToBP_Character (Game|GetPlayerCharacter 0)))
    (Transformation|SetActorRotation (Math|Rotator|FindLookatRotation (Transformation|GetActorLocation) (Transformation|GetActorLocation _asbp_character)))))

(event Custom|Visibility
  (bind _spotlight (Variables|Default|GetSpotLight))
  (if (Variables|Default|GetIsActive)
    (Rendering|SetVisibility _spotlight true false)
    (else
      (Rendering|SetVisibility _spotlight false false))))

(event EventBeginPlay
  (Rendering|Components|TextRender|SetText (Variables|Default|GetTextRender) (Variables|Default|GetText))
  (Rendering|Components|TextRender|SetText (Variables|Default|GetTextRender1) (Variables|Default|GetText1))
  (CallFunction|Visibility))

(event Collision|EventActorBeginOverlap
  (params (OtherActor :type Actor%20Object%20Reference)))

(event EventTick
  (params (DeltaSeconds :type Float%20%28single-precision%29))
  (CallFunction|FollowCharacter))

(fn ConstructionScript)