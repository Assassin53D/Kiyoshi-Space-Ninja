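; BP_DoorHorizontalAutoR is an automatic door that slides horizontally when a BP_Character enters UpCollision and returns when one leaves DownCollision.
; The construction script stores the Cube's start position and a target offset along world X.
; A timeline plays or reverses between them, feeding its track into VInterpTo's DeltaTime as a blend alpha.
; Overlaps swap the open and close sounds, and both stop when the timeline finishes.
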(event OnComponentBeginOverlap(UpCollision)
  (params (OverlappedComponent :type Primitive%20Component%20Object%20Reference) (OtherActor :type Actor%20Object%20Reference) (OtherComp :type Primitive%20Component%20Object%20Reference) (OtherBodyIndex :type Integer) (bFromSweep :type Boolean) (SweepResult :type Hit%20Result%20Structure%20%28by%20ref%29))
  (Utilities|Casting|CastToBP_Character OtherActor)
  (Components|Activation|Activate (Variables|Default|GetAudio_DoorOpen) false)
  (Components|Activation|Deactivate (Variables|Default|GetAudio_DoorClose))
  (bind _newtrack_1 (Timeline|Timeline_0 Play)
    (:Update
      (Transformation|SetWorldLocation (Variables|Default|GetCube) (Math|Interpolation|VInterpTo (Variables|Default|GetDoorDown) (Variables|Default|GetDoorUp) _newtrack_1 1.0) false false))
    (:Finished
      (Components|Activation|Deactivate (Variables|Default|GetAudio_DoorClose))
      (Components|Activation|Deactivate (Variables|Default|GetAudio_DoorOpen)))))

(event OnComponentEndOverlap(DownCollision)
  (params (OverlappedComponent :type Primitive%20Component%20Object%20Reference) (OtherActor :type Actor%20Object%20Reference) (OtherComp :type Primitive%20Component%20Object%20Reference) (OtherBodyIndex :type Integer))
  (Utilities|Casting|CastToBP_Character OtherActor)
  (Components|Activation|Activate (Variables|Default|GetAudio_DoorClose) false)
  (Components|Activation|Deactivate (Variables|Default|GetAudio_DoorOpen))
  (bind _newtrack_1 (Timeline|Timeline_0 Reverse)
    (:Update
      (Transformation|SetWorldLocation (Variables|Default|GetCube) (Math|Interpolation|VInterpTo (Variables|Default|GetDoorDown) (Variables|Default|GetDoorUp) _newtrack_1 1.0) false false))
    (:Finished
      (Components|Activation|Deactivate (Variables|Default|GetAudio_DoorClose))
      (Components|Activation|Deactivate (Variables|Default|GetAudio_DoorOpen)))))

(event EventBeginPlay)

(event Collision|EventActorBeginOverlap
  (params (OtherActor :type Actor%20Object%20Reference)))

(event EventTick
  (params (DeltaSeconds :type Float%20%28single-precision%29)))

(fn ConstructionScript
  (bind _output_get (Variables|Default|SetDoorDown (Transformation|GetWorldLocation (Variables|Default|GetCube))))
  (Variables|Default|SetDoorUp (Math|Vector|MakeVector (+ (.X (Math|Vector|BreakVector _output_get)) 3e+02) (.Y (Math|Vector|BreakVector _output_get)) (.Z (Math|Vector|BreakVector _output_get)))))