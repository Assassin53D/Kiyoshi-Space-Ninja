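; Switch-driven platform that slides its Cube horizontally along X to an offset point and back, once IsActivated is true.
; Construction script caches both endpoints, and Tick polls the flag through DoOnce nodes that are never reset, allowing one trip out and, after a delay, one return.
; A timeline played then reversed feeds its track into VInterpTo as DeltaTime between the fixed endpoints, setting ReachedTheTop when finished.
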(event Custom|GoingOutside
  (Variables|Default|SetGoing%20Down false)
  (bind _newtrack_1 (Timeline|Timeline_0 Reverse)
    (:Update
      (Transformation|SetWorldLocation (Variables|Default|GetCube) (Math|Interpolation|VInterpTo (Variables|Default|GetDoorOutside) (Variables|Default|GetDoorInside) _newtrack_1 1.0) false false))
    (:Finished
      (if (Variables|Default|GetGoing%20Down)
        (Variables|Default|SetReachedTheTop false)
        (else
          (Variables|Default|SetReachedTheTop true))))))

(event Custom|GoingInside
  (Variables|Default|SetGoing%20Down true)
  (bind _newtrack_1 (Timeline|Timeline_0 Play)
    (:Update
      (Transformation|SetWorldLocation (Variables|Default|GetCube) (Math|Interpolation|VInterpTo (Variables|Default|GetDoorOutside) (Variables|Default|GetDoorInside) _newtrack_1 1.0) false false))
    (:Finished
      (if (Variables|Default|GetGoing%20Down)
        (Variables|Default|SetReachedTheTop false)
        (else
          (Variables|Default|SetReachedTheTop true))))))

(event Custom|PlatformPosition
  (if (Variables|Default|GetIsActivated)
    (Utilities|FlowControl|DoOnce false
      (:Completed
        (CallFunction|GoingInside)
        (Utilities|FlowControl|Delay 2.0)
        (Utilities|FlowControl|DoOnce false
          (:Completed
            (CallFunction|GoingOutside)))))))

(event EventBeginPlay)

(event Collision|EventActorBeginOverlap
  (params (OtherActor :type Actor%20Object%20Reference)))

(event EventTick
  (params (DeltaSeconds :type Float%20%28single-precision%29))
  (CallFunction|PlatformPosition))

(fn ConstructionScript
  (bind _output_get (Variables|Default|SetDoorOutside (Transformation|GetWorldLocation (Variables|Default|GetCube))))
  (Variables|Default|SetDoorInside (Math|Vector|MakeVector (+ (.X (Math|Vector|BreakVector _output_get)) 3.5e+02) (.Y (Math|Vector|BreakVector _output_get)) (.Z (Math|Vector|BreakVector _output_get)))))