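; BP_InvisibilityStation is an environment zone that turns an overlapping BP_Character invisible.
; Entering its mesh plays a sound and disables throw, deflect and dash, which return on exit.
; Entry opens a Tick-driven gate that keeps restarting a retriggerable delay, and exit closes it.
; Invisibility thus lingers for InvisibilityDuration after leaving, then ends on the last character to exit via PlayEndInvis.
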(event OnComponentBeginOverlap(StaticMesh1)
  (params (OverlappedComponent :type Primitive%20Component%20Object%20Reference) (OtherActor :type Actor%20Object%20Reference) (OtherComp :type Primitive%20Component%20Object%20Reference) (OtherBodyIndex :type Integer) (bFromSweep :type Boolean) (SweepResult :type Hit%20Result%20Structure%20%28by%20ref%29))
  (bind _asbp_character (Utilities|Casting|CastToBP_Character OtherActor))
  (Variables|/Game/Ninja/Blueprints/Character/BP_Character.BP_Character_C|SetIsInvisible _asbp_character true)
  (Variables|/Game/Ninja/Blueprints/Character/BP_Character.BP_Character_C|SetCanThrow _asbp_character false)
  (Variables|/Game/Ninja/Blueprints/Character/BP_Character.BP_Character_C|SetCanDeflect _asbp_character false)
  (Variables|/Game/Ninja/Blueprints/Character/BP_Character.BP_Character_C|SetCanDash _asbp_character false)
  (Variables|/Game/Ninja/Blueprints/Character/BP_Character.BP_Character_C|SetIsDeflecting _asbp_character false)
  (Audio|PlaySoundatLocation "/Game/Ninja/Audio/SFX_InvisibilityIn_001_Cue.SFX_InvisibilityIn_001_Cue" (Transformation|GetActorLocation _asbp_character))
  (Utilities|FlowControl|Gate true) ; enters at Open
)

(event OnComponentEndOverlap(StaticMesh1)
  (params (OverlappedComponent :type Primitive%20Component%20Object%20Reference) (OtherActor :type Actor%20Object%20Reference) (OtherComp :type Primitive%20Component%20Object%20Reference) (OtherBodyIndex :type Integer))
  (bind _asbp_character (Utilities|Casting|CastToBP_Character OtherActor))
  (Variables|/Game/Ninja/Blueprints/Character/BP_Character.BP_Character_C|SetCanThrow _asbp_character true)
  (Variables|/Game/Ninja/Blueprints/Character/BP_Character.BP_Character_C|SetCanDeflect _asbp_character true)
  (Variables|/Game/Ninja/Blueprints/Character/BP_Character.BP_Character_C|SetCanDash _asbp_character true)
  (Utilities|FlowControl|Gate true) ; enters at Close
)

(event EventBeginPlay)

(event Collision|EventActorBeginOverlap
  (params (OtherActor :type Actor%20Object%20Reference)))

(event EventTick
  (params (DeltaSeconds :type Float%20%28single-precision%29))
  (Utilities|FlowControl|Gate true
    (:Exit
      (Utilities|FlowControl|RetriggerableDelay (Variables|Default|GetInvisibilityDuration))
      (Default|PlayEndInvis (stale OnComponentEndOverlap(StaticMesh1) _asbp_character))
      (Variables|/Game/Ninja/Blueprints/Character/BP_Character.BP_Character_C|SetIsInvisible (stale OnComponentEndOverlap(StaticMesh1) _asbp_character) false))))

(fn ConstructionScript)