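; BP_Crates is an environment crate that is destroyed when hit by a kunai.
; A FirstPersonProjectile overlapping Box destroys the projectile, plays a kunai impact sound at the box's location, then destroys the crate.
; A second volume, Box1, turns off physics simulation on the Crate component while BP_Character overlaps it and turns it back on when the character leaves.
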(event OnComponentBeginOverlap(Box)
  (params (OverlappedComponent :type Primitive%20Component%20Object%20Reference) (OtherActor :type Actor%20Object%20Reference) (OtherComp :type Primitive%20Component%20Object%20Reference) (OtherBodyIndex :type Integer) (bFromSweep :type Boolean) (SweepResult :type Hit%20Result%20Structure%20%28by%20ref%29))
  ;[1 1 1] Kuinai hitting Crate
  (bind _asfirst_person_projectile (Utilities|Casting|CastToFirstPersonProjectile OtherActor))
  (Actor|DestroyActor _asfirst_person_projectile)
  (Audio|PlaySoundatLocation "/Game/Ninja/Audio/SFX_KunaiHittingBox_001_Cue.SFX_KunaiHittingBox_001_Cue" (Transformation|GetWorldLocation (Variables|Default|GetBox)))
  (Actor|DestroyActor))

(event OnComponentEndOverlap(Box1)
  (params (OverlappedComponent :type Primitive%20Component%20Object%20Reference) (OtherActor :type Actor%20Object%20Reference) (OtherComp :type Primitive%20Component%20Object%20Reference) (OtherBodyIndex :type Integer))
  (Utilities|Casting|CastToBP_Character OtherActor)
  (Physics|SetSimulatePhysics (Variables|Default|GetCrate) true))

(event OnComponentBeginOverlap(Box1)
  (params (OverlappedComponent :type Primitive%20Component%20Object%20Reference) (OtherActor :type Actor%20Object%20Reference) (OtherComp :type Primitive%20Component%20Object%20Reference) (OtherBodyIndex :type Integer) (bFromSweep :type Boolean) (SweepResult :type Hit%20Result%20Structure%20%28by%20ref%29))
  (Utilities|Casting|CastToBP_Character OtherActor)
  (Physics|SetSimulatePhysics (Variables|Default|GetCrate) false))

(event EventBeginPlay)

(event Collision|EventActorBeginOverlap
  (params (OtherActor :type Actor%20Object%20Reference)))

(event EventTick
  (params (DeltaSeconds :type Float%20%28single-precision%29)))

(fn ConstructionScript)