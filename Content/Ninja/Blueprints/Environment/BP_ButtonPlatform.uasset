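; BP_ButtonPlatform is a pressure-button platform that is active while a character or crate rests on it.
; Box begin and end overlaps track BP_Character and BP_Crates with separate landed flags that together drive IsActivated.
; IsActivated clears when one leaves while the other is absent.
; Each type uses a single boolean instead of a count, and the graph only sets state, with no visible response.
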(event OnComponentBeginOverlap(Box)
  (params (OverlappedComponent :type Primitive%20Component%20Object%20Reference) (OtherActor :type Actor%20Object%20Reference) (OtherComp :type Primitive%20Component%20Object%20Reference) (OtherBodyIndex :type Integer) (bFromSweep :type Boolean) (SweepResult :type Hit%20Result%20Structure%20%28by%20ref%29))
  (Utilities|FlowControl|Sequence
    (:then_0
      (Utilities|Casting|CastToBP_Character OtherActor)
      (Variables|Default|SetPlayerHasLanded true)
      (if (not (Variables|Default|GetCrateHasLanded))
        (Variables|Default|SetIsActivated true :!label _label)))
    (:then_1
      (Utilities|Casting|CastToBP_Crates OtherActor)
      (Variables|Default|SetCrateHasLanded true)
      (goto _label))))

(event OnComponentEndOverlap(Box)
  (params (OverlappedComponent :type Primitive%20Component%20Object%20Reference) (OtherActor :type Actor%20Object%20Reference) (OtherComp :type Primitive%20Component%20Object%20Reference) (OtherBodyIndex :type Integer))
  (Utilities|FlowControl|Sequence
    (:then_0
      (Utilities|Casting|CastToBP_Character OtherActor)
      (Variables|Default|SetPlayerHasLanded false)
      (if (not (Variables|Default|GetCrateHasLanded))
        (Variables|Default|SetIsActivated false :!label _label)))
    (:then_1
      (Utilities|Casting|CastToBP_Crates OtherActor)
      (if (Variables|Default|GetPlayerHasLanded)
        (Variables|Default|SetCrateHasLanded false)
        (else
          (Variables|Default|SetCrateHasLanded false)
          (goto _label))))))

(event EventBeginPlay)

(event Collision|EventActorBeginOverlap
  (params (OtherActor :type Actor%20Object%20Reference)))

(event EventTick
  (params (DeltaSeconds :type Float%20%28single-precision%29)))

(fn ConstructionScript)