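; Checkpoint trigger actor that saves the player's progress and can unlock abilities in the ninja game.
; A Player-tagged overlap creates a SaveValues object and, once only, writes health, kunai count and location to a fixed save slot.
; Box1 enables flagged wall climb, kunai text, dash and deflect with their HUD widgets.
; Box2 briefly flags the character as in checkpoint, then destroys itself; construction sizes Box from TriggerResize.
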(event OnComponentBeginOverlap(Box1)
  (params (OverlappedComponent :type Primitive%20Component%20Object%20Reference) (OtherActor :type Actor%20Object%20Reference) (OtherComp :type Primitive%20Component%20Object%20Reference) (OtherBodyIndex :type Integer) (bFromSweep :type Boolean) (SweepResult :type Hit%20Result%20Structure%20%28by%20ref%29))
  (bind _asbp_character (Utilities|Casting|CastToBP_Character OtherActor))
  (Utilities|FlowControl|Sequence
    (:then_0
      (if (Variables|Default|GetHasWallClimb)
        (Variables|/Game/Ninja/Blueprints/Character/BP_Character.BP_Character_C|SetCanWallClimb _asbp_character true)
        (Widget|SetVisibility (Variables|/Game/Ninja/UI/PlayerWidget.PlayerWidget_C|GetGripBar (Variables|/Game/Ninja/Blueprints/Character/BP_Character.BP_Character_C|GetGameUIRef _asbp_character)) "Visible")))
    (:then_1
      (if (Variables|Default|GetHasKunai)
        (Variables|/Game/Ninja/Blueprints/Character/BP_Character.BP_Character_C|SetShowKunaiText _asbp_character true)
        (Widget|SetVisibility (Variables|/Game/Ninja/UI/PlayerWidget.PlayerWidget_C|GetKunaiImage (Variables|/Game/Ninja/Blueprints/Character/BP_Character.BP_Character_C|GetGameUIRef _asbp_character)) "Visible")))
    (:then_2
      (if (Variables|Default|GetHasDash)
        (Variables|/Game/Ninja/Blueprints/Character/BP_Character.BP_Character_C|SetCanDash _asbp_character true)
        (Widget|SetVisibility (Variables|/Game/Ninja/UI/PlayerWidget.PlayerWidget_C|GetDashBar (Variables|/Game/Ninja/Blueprints/Character/BP_Character.BP_Character_C|GetGameUIRef _asbp_character)) "Visible")))
    (:then_3
      (if (Variables|Default|GetHasDeflect)
        (Variables|/Game/Ninja/Blueprints/Character/BP_Character.BP_Character_C|SetCanDeflect _asbp_character true)
        (Widget|SetVisibility (Variables|/Game/Ninja/UI/PlayerWidget.PlayerWidget_C|GetDeflectBar (Variables|/Game/Ninja/Blueprints/Character/BP_Character.BP_Character_C|GetGameUIRef _asbp_character)) "Visible")))))

(event OnComponentBeginOverlap(Box2)
  (params (OverlappedComponent :type Primitive%20Component%20Object%20Reference) (OtherActor :type Actor%20Object%20Reference) (OtherComp :type Primitive%20Component%20Object%20Reference) (OtherBodyIndex :type Integer) (bFromSweep :type Boolean) (SweepResult :type Hit%20Result%20Structure%20%28by%20ref%29))
  (bind _asbp_character (Utilities|Casting|CastToBP_Character OtherActor))
  (Variables|/Game/Ninja/Blueprints/Character/BP_Character.BP_Character_C|SetIsInCheckpoint _asbp_character true)
  (Components|DestroyComponent (Variables|Default|GetBox2))
  (Utilities|FlowControl|Delay 2.0)
  (Variables|/Game/Ninja/Blueprints/Character/BP_Character.BP_Character_C|SetIsInCheckpoint _asbp_character false))

(event EventBeginPlay)

(event EventTick
  (params (DeltaSeconds :type Float%20%28single-precision%29)))

(event Collision|EventActorBeginOverlap
  (params (OtherActor :type Actor%20Object%20Reference))
  (if (Actor|ActorHasTag OtherActor "Player")
    (Utilities|FlowControl|Sequence
      (:then_0
        (bind _returnvalue (SaveGame|CreateSaveGameObject "/Game/Ninja/Blueprints/SaveProgram/SaveValues.SaveValues_C"))
        (bind _assave_values (Utilities|Casting|CastToSaveValues _returnvalue))
        (Variables|Default|SetSave _assave_values)
        (bind _asbp_character (Utilities|Casting|CastToBP_Character (Game|GetPlayerCharacter 0)))
        (Variables|Default|SetCharacter _asbp_character)
        (Variables|Default|SetEnabledCheckpoint true)
        (if (Variables|Default|GetEnabledCheckpoint)
          (Utilities|FlowControl|DoOnce false
            (:Completed
              (Variables|/Game/Ninja/Blueprints/SaveProgram/SaveValues.SaveValues_C|SetHealth (Variables|Default|GetSave) (Variables|/Game/Ninja/Blueprints/Character/BP_Character.BP_Character_C|GetHealth (Variables|Default|GetCharacter)))
              (Variables|/Game/Ninja/Blueprints/SaveProgram/SaveValues.SaveValues_C|SetKunaiAmount (Variables|Default|GetSave) (Variables|/Game/Ninja/Blueprints/Character/BP_Character.BP_Character_C|GetKunai%20Amount (Variables|Default|GetCharacter)))
              (Variables|/Game/Ninja/Blueprints/SaveProgram/SaveValues.SaveValues_C|SetCheckpoint (Variables|Default|GetSave) (Transformation|GetActorLocation (Variables|Default|GetCharacter)))
              (Variables|/Game/Ninja/Blueprints/SaveProgram/SaveValues.SaveValues_C|SetNewLevel (Variables|Default|GetSave) false)
              (SaveGame|SaveGametoSlot (Variables|Default|GetSave) "Save001"))))))))

(fn ConstructionScript
  (Components|Box|SetBoxExtent (Variables|Default|GetBox) (Variables|Default|GetTriggerResize) true)
  (if (Variables|Default|GetEnabledCheckpoint)
    _))