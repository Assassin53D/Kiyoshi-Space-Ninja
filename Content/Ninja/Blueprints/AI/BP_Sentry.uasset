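; BP_Sentry is a patrolling AI enemy that chases a seen BP_Character and self-destructs.
; It loops through up to ten patrol points using chained AIMoveTo calls with random delays.
; Sighting turns its spotlight from green to red and starts a three-second fuse as the chase begins, then spawns BP_SentryExplosion.
; A FirstPersonProjectile hit destroys it without exploding; the per-tick animation hook is empty.
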(event OnComponentBeginOverlap(Sphere1)
  (params (OverlappedComponent :type Primitive%20Component%20Object%20Reference) (OtherActor :type Actor%20Object%20Reference) (OtherComp :type Primitive%20Component%20Object%20Reference) (OtherBodyIndex :type Integer) (bFromSweep :type Boolean) (SweepResult :type Hit%20Result%20Structure%20%28by%20ref%29))
  (Utilities|Casting|CastToFirstPersonProjectile OtherActor)
  (Variables|Default|SetIsShot true)
  (Actor|DestroyActor))

(event OnSeePawn(PawnSensing)
  (params (Pawn :type Pawn%20Object%20Reference))
  (bind _asbp_character (Utilities|Casting|CastToBP_Character Pawn))
  (Variables|Default|SetIsChasing true)
  (AI|AIMoveTo self "0.000000,0.000000,0.000000" _asbp_character 5.0 false
    (:then
      (CallFunction|Explosion))))

(event Custom|Explosion
  (Utilities|FlowControl|Delay 3.0)
  (if (not (Variables|Default|GetIsShot))
    (Game|SpawnActorfromClass "/Game/Ninja/Blueprints/AI/BP_SentryExplosion.BP_SentryExplosion_C" (Transformation|GetWorldTransform (Variables|Default|GetArrow1)) "Undefined" 0 0)
    (Actor|DestroyActor)))

(event Custom|Lights
  (bind _spotlight (Variables|Default|GetSpotLight))
  (if (Variables|Default|GetIsChasing)
    (Rendering|Components|Light|SetLightColor _spotlight "(R=1.000000,G=0.000000,B=0.000000,A=1.000000)" true)
    (else
      (Rendering|Components|Light|SetLightColor _spotlight "(R=0.000000,G=1.000000,B=0.019382,A=1.000000)" true))))

(event Custom|AnimationChange)

(event Custom|Patrol
  (AI|AIMoveTo self "0,0.000000, 0" (Variables|Default|GetPatrolPoint_0) 5e+01 false
    (:OnSuccess
      (if (>= (Variables|Default|GetAmountpatrolpoints) 2)
        (Utilities|FlowControl|Delay (Math|Random|RandomFloatinRange (Variables|Default|GetDelay0) (Variables|Default|GetDelay1)))
        (AI|AIMoveTo self "0, 0, 0" (Variables|Default|GetPatrolPoint_1) 5e+01 false
          (:OnSuccess
            (if (>= (Variables|Default|GetAmountpatrolpoints) 3)
              (Utilities|FlowControl|Delay (Math|Random|RandomFloatinRange (Variables|Default|GetDelay0) (Variables|Default|GetDelay1)))
              (AI|AIMoveTo self "0, 0, 0" (Variables|Default|GetPatrolPoint_2) 5e+01 false
                (:OnSuccess
                  (if (>= (Variables|Default|GetAmountpatrolpoints) 4)
                    (Utilities|FlowControl|Delay (Math|Random|RandomFloatinRange (Variables|Default|GetDelay0) (Variables|Default|GetDelay1)))
                    (AI|AIMoveTo self "0, 0, 0" (Variables|Default|GetPatrolPoint_3) 5e+01 false
                      (:OnSuccess
                        (if (>= (Variables|Default|GetAmountpatrolpoints) 5)
                          (Utilities|FlowControl|Delay (Math|Random|RandomFloatinRange (Variables|Default|GetDelay0) (Variables|Default|GetDelay1)))
                          (AI|AIMoveTo self "0, 0, 0" (Variables|Default|GetPatrolPoint_4) 5e+01 false
                            (:OnSuccess
                              (if (>= (Variables|Default|GetAmountpatrolpoints) 6)
                                (Utilities|FlowControl|Delay (Math|Random|RandomFloatinRange (Variables|Default|GetDelay0) (Variables|Default|GetDelay1)))
                                (AI|AIMoveTo self "0, 0, 0" (Variables|Default|GetPatrolPoint_5) 5e+01 false
                                  (:OnSuccess
                                    (if (>= (Variables|Default|GetAmountpatrolpoints) 7)
                                      (Utilities|FlowControl|Delay (Math|Random|RandomFloatinRange (Variables|Default|GetDelay0) (Variables|Default|GetDelay1)))
                                      (AI|AIMoveTo self "0, 0, 0" (Variables|Default|GetPatrolPoint_6) 5e+01 false
                                        (:OnSuccess
                                          (if (>= (Variables|Default|GetAmountpatrolpoints) 8)
                                            (Utilities|FlowControl|Delay (Math|Random|RandomFloatinRange (Variables|Default|GetDelay0) (Variables|Default|GetDelay1)))
                                            (AI|AIMoveTo self "0, 0, 0" (Variables|Default|GetPatrolPoint_7) 5e+01 false
                                              (:OnSuccess
                                                (if (>= (Variables|Default|GetAmountpatrolpoints) 9)
                                                  (Utilities|FlowControl|Delay (Math|Random|RandomFloatinRange (Variables|Default|GetDelay0) (Variables|Default|GetDelay1)))
                                                  (AI|AIMoveTo self "0, 0, 0" (Variables|Default|GetPatrolPoint_8) 5e+01 false
                                                    (:OnSuccess
                                                      (if (>= (Variables|Default|GetAmountpatrolpoints) 10)
                                                        (Utilities|FlowControl|Delay (Math|Random|RandomFloatinRange (Variables|Default|GetDelay0) (Variables|Default|GetDelay1)))
                                                        (AI|AIMoveTo self "0, 0,0.000000" (Variables|Default|GetPatrolPoint_9) 5e+01 false
                                                          (:OnSuccess
                                                            _)))))))))))))))))))))))))))
      (Utilities|FlowControl|Delay (Math|Random|RandomFloatinRange (Variables|Default|GetDelay0) (Variables|Default|GetDelay1)))
      (CallFunction|Patrol))))

(event EventTick
  (params (DeltaSeconds :type Float%20%28single-precision%29))
  (CallFunction|Lights)
  (CallFunction|AnimationChange))

(event EventBeginPlay
  (CallFunction|Patrol))

(fn ConstructionScript)