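; BP_SentryExplosion is a short-lived explosion actor that damages what its sphere overlaps.
; On sphere overlap, it reduces a BP_Character's health and launches it upward, guarded by a DoOnce so this happens only once per explosion.
; Any overlapping BP_DoorVerticalExplosion is destroyed.
; After a brief delay from BeginPlay, it plays the sentry explosion sound at its location and destroys itself.
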(event OnComponentBeginOverlap(Sphere)
  (params (OverlappedComponent :type Primitive%20Component%20Object%20Reference) (OtherActor :type Actor%20Object%20Reference) (OtherComp :type Primitive%20Component%20Object%20Reference) (OtherBodyIndex :type Integer) (bFromSweep :type Boolean) (SweepResult :type Hit%20Result%20Structure%20%28by%20ref%29))
  (Utilities|FlowControl|Sequence
    (:then_0
      (bind _asbp_character (Utilities|Casting|CastToBP_Character OtherActor))
      (Utilities|FlowControl|DoOnce false
        (:Completed
          (Variables|/Game/Ninja/Blueprints/Character/BP_Character.BP_Character_C|SetHealth _asbp_character (- (Variables|/Game/Ninja/Blueprints/Character/BP_Character.BP_Character_C|GetHealth _asbp_character) 0.5))
          (Character|LaunchCharacter _asbp_character "0, 0,750.000000" false false))))
    (:then_1
      (bind _asbp_door_vertical_explosion (Utilities|Casting|CastToBP_DoorVerticalExplosion OtherActor))
      (Actor|DestroyActor _asbp_door_vertical_explosion))))

(event EventBeginPlay
  (Utilities|FlowControl|Delay 0.2)
  (Audio|PlaySoundatLocation "/Game/Ninja/Audio/SFX_SentryExplode_001_Cue.SFX_SentryExplode_001_Cue" (Transformation|GetWorldLocation (Variables|Default|GetScene)))
  (Actor|DestroyActor))

(event Collision|EventActorBeginOverlap
  (params (OtherActor :type Actor%20Object%20Reference)))

(event EventTick
  (params (DeltaSeconds :type Float%20%28single-precision%29)))

(fn ConstructionScript)