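; BP_AIDefense is a defensive AI unit whose shield drops temporarily when a projectile hits its Box trigger.
; Tick syncs the shield's collision and visibility to IsActive, setting the idle animation once per activation.
; A first-person projectile (destroyed on contact) or deflected turret projectile clears IsActive and plays stun animation and audio.
; Retriggerable delays then play the reboot animation and audio before restoring the shield.
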(event OnComponentBeginOverlap(Box)
  (params (OverlappedComponent :type Primitive%20Component%20Object%20Reference) (OtherActor :type Actor%20Object%20Reference) (OtherComp :type Primitive%20Component%20Object%20Reference) (OtherBodyIndex :type Integer) (bFromSweep :type Boolean) (SweepResult :type Hit%20Result%20Structure%20%28by%20ref%29))
  (Utilities|FlowControl|Sequence
    (:then_0
      (bind _asfirst_person_projectile (Utilities|Casting|CastToFirstPersonProjectile OtherActor))
      (Actor|DestroyActor _asfirst_person_projectile))
    (:then_1
      (Utilities|Casting|CastToBP_TurretProjectileDeflected OtherActor)))
  (Variables|Default|SetIsActive false)
  (Components|Animation|PlayAnimation (Variables|Default|GetSkeletalMesh) "/Game/Ninja/Models/Robots/Defense/Anim_DefenceStun_Montage.Anim_DefenceStun_Montage" false)
  (Components|Activation|Activate (Variables|Default|GetAudio_Stun) false)
  (Components|Activation|Deactivate (Variables|Default|GetAudio_Reboot))
  (Utilities|FlowControl|Sequence
    (:then_0
      (Utilities|FlowControl|RetriggerableDelay 2.0)
      (Utilities|FlowControl|DoOnce false :!label _label
        (:Completed
          (Components|Animation|PlayAnimation (Variables|Default|GetSkeletalMesh) "/Game/Ninja/Models/Robots/Defense/Anim_DefenceShield_Montage.Anim_DefenceShield_Montage" false)
          (Components|Activation|Activate (Variables|Default|GetAudio_Reboot) false)
          (Components|Activation|Deactivate (Variables|Default|GetAudio_Stun)))))
    (:then_1
      (Utilities|FlowControl|RetriggerableDelay 3.2)
      (Variables|Default|SetIsActive true)
      (goto _label Reset))))

(event Custom|ShieldActivation
  (bind _shield (Variables|Default|GetShield))
  (if (Variables|Default|GetIsActive)
    (Collision|SetCollisionEnabled _shield "QueryAndPhysics")
    (Rendering|SetVisibility _shield true false)
    (Utilities|FlowControl|DoOnce false :!label _label
      (:Completed
        (Components|Animation|OverrideAnimationData (Variables|Default|GetSkeletalMesh) "/Game/Ninja/Models/Robots/Defense/Anim_DefenceIdle.Anim_DefenceIdle" true true 0.0 1.0)))
    (else
      (Collision|SetCollisionEnabled _shield "NoCollision")
      (Rendering|SetVisibility _shield false false)
      (goto _label Reset))))

(event EventBeginPlay)

(event Collision|EventActorBeginOverlap
  (params (OtherActor :type Actor%20Object%20Reference)))

(event EventTick
  (params (DeltaSeconds :type Float%20%28single-precision%29))
  (CallFunction|ShieldActivation))

(fn ConstructionScript)