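; Enemy AI pawn that patrols, chases a seen BP_Character and damages the player at close range.
; From BeginPlay, chained AI MoveTo calls visit up to ten points with random pauses, then loop; PawnSensing issues a move toward the character.
; Box1 overlaps flag the player in range and register projectile hits, which lower Health until the enemy is destroyed.
; While flagged, Tick-driven attacks use a Delay to space out damage.
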(event OnComponentEndOverlap(Box2)
  (params (OverlappedComponent :type Primitive%20Component%20Object%20Reference) (OtherActor :type Actor%20Object%20Reference) (OtherComp :type Primitive%20Component%20Object%20Reference) (OtherBodyIndex :type Integer)))

(event OnComponentEndOverlap(Box1)
  (params (OverlappedComponent :type Primitive%20Component%20Object%20Reference) (OtherActor :type Actor%20Object%20Reference) (OtherComp :type Primitive%20Component%20Object%20Reference) (OtherBodyIndex :type Integer))
  (Utilities|Casting|CastToBP_Character OtherActor)
  (Variables|Default|SetEnemyinrange false))

(event OnComponentBeginOverlap(Box1)
  (params (OverlappedComponent :type Primitive%20Component%20Object%20Reference) (OtherActor :type Actor%20Object%20Reference) (OtherComp :type Primitive%20Component%20Object%20Reference) (OtherBodyIndex :type Integer) (bFromSweep :type Boolean) (SweepResult :type Hit%20Result%20Structure%20%28by%20ref%29))
  (Utilities|FlowControl|Sequence
    (:then_0
      (Utilities|Casting|CastToFirstPersonProjectile OtherActor)
      (CallFunction|TakeDamage self))
    (:then_1
      (Utilities|Casting|CastToBP_Character OtherActor)
      (Variables|Default|SetEnemyinrange true))))

(event OnComponentBeginOverlap(Box2)
  (params (OverlappedComponent :type Primitive%20Component%20Object%20Reference) (OtherActor :type Actor%20Object%20Reference) (OtherComp :type Primitive%20Component%20Object%20Reference) (OtherBodyIndex :type Integer) (bFromSweep :type Boolean) (SweepResult :type Hit%20Result%20Structure%20%28by%20ref%29)))

(event OnSeePawn(PawnSensing)
  (params (Pawn :type Pawn%20Object%20Reference))
  (bind _asbp_character (Utilities|Casting|CastToBP_Character Pawn))
  (AI|AIMoveTo self "0.000000,0.000000,0.000000" _asbp_character 5.0 false))

(event Custom|Death
  (if (<= (Variables|Default|GetHealth) 0)
    (Actor|DestroyActor self)))

(event Custom|deal%20damage
  (if (Variables|Default|Getenemyinrange)
    (bind _asbp_character (Utilities|Casting|CastToBP_Character (Game|Player|GetPlayerPawn 0)))
    (Utilities|FlowControl|Delay 3.0)
    (bind _output_get (Variables|/Game/Ninja/Blueprints/Character/BP_Character.BP_Character_C|SetHealth _asbp_character (- (Variables|/Game/Ninja/Blueprints/Character/BP_Character.BP_Character_C|GetHealth _asbp_character) 10)))
    (Development|PrintString (Utilities|String|ToString(Integer) _output_get))
    (Default|Death _asbp_character)))

(event Custom|Take%20Damage
  (Development|PrintString (Utilities|String|ToString(Integer) (Variables|Default|GetHealth)))
  (Variables|Default|SetHealth (- (Variables|Default|GetHealth) 10))
  (CallFunction|Death self))

(event Custom|Patrol
  (AI|AIMoveTo self (Variables|Default|GetPatrol%20Point%201) 0 5e+01 false
    (:OnSuccess
      (if (>= (Variables|Default|GetAmountpatrolpoints) 2)
        (Utilities|FlowControl|Delay (Math|Random|RandomFloatinRange 2.0 3.0))
        (AI|AIMoveTo self (Variables|Default|Getpatrol%20point%202) 0 5e+01 false
          (:OnSuccess
            (if (>= (Variables|Default|GetAmountpatrolpoints) 3)
              (Utilities|FlowControl|Delay (Math|Random|RandomFloatinRange 2.0 3.0))
              (AI|AIMoveTo self (Variables|Default|Getpatrol%20point%203) 0 5e+01 false
                (:OnSuccess
                  (if (>= (Variables|Default|GetAmountpatrolpoints) 4)
                    (Utilities|FlowControl|Delay (Math|Random|RandomFloatinRange 2.0 3.0))
                    (AI|AIMoveTo self (Variables|Default|Getpatrol%20point%204) 0 5e+01 false
                      (:OnSuccess
                        (if (>= (Variables|Default|GetAmountpatrolpoints) 5)
                          (Utilities|FlowControl|Delay (Math|Random|RandomFloatinRange 2.0 3.0))
                          (AI|AIMoveTo self (Variables|Default|Getpatrol%20point%205) 0 5e+01 false
                            (:OnSuccess
                              (if (>= (Variables|Default|GetAmountpatrolpoints) 6)
                                (Utilities|FlowControl|Delay (Math|Random|RandomFloatinRange 2.0 3.0))
                                (AI|AIMoveTo self (Variables|Default|Getpatrol%20point%206) 0 5e+01 false
                                  (:OnSuccess
                                    (if (>= (Variables|Default|GetAmountpatrolpoints) 7)
                                      (Utilities|FlowControl|Delay (Math|Random|RandomFloatinRange 2.0 3.0))
                                      (AI|AIMoveTo self (Variables|Default|Getpatrol%20point%207) 0 5e+01 false
                                        (:OnSuccess
                                          (if (>= (Variables|Default|GetAmountpatrolpoints) 8)
                                            (Utilities|FlowControl|Delay (Math|Random|RandomFloatinRange 2.0 3.0))
                                            (AI|AIMoveTo self (Variables|Default|Getpatrol%20point%208) 0 5e+01 false
                                              (:OnSuccess
                                                (if (>= (Variables|Default|GetAmountpatrolpoints) 9)
                                                  (Utilities|FlowControl|Delay (Math|Random|RandomFloatinRange 2.0 3.0))
                                                  (AI|AIMoveTo self (Variables|Default|Getpatrol%20point%209) 0 5e+01 false
                                                    (:OnSuccess
                                                      (if (>= (Variables|Default|GetAmountpatrolpoints) 10)
                                                        (Utilities|FlowControl|Delay (Math|Random|RandomFloatinRange 2.0 3.0))
                                                        (AI|AIMoveTo self (Variables|Default|Getpatrol%20point%2010) 0 5e+01 false
                                                          (:OnSuccess
                                                            _)))))))))))))))))))))))))))
      (Utilities|FlowControl|Delay 3.0)
      (CallFunction|Patrol))))

(event EventBeginPlay
  (CallFunction|Patrol))

(event EventTick
  (params (DeltaSeconds :type Float%20%28single-precision%29))
  (CallFunction|DealDamage))

(fn ConstructionScript)