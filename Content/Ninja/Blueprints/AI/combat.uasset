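; Enemy AI pawn that chases BP_Character, kills it after contact and can be shot down.
; Entering Box2 starts an AIMoveTo chase, while leaving it sends the pawn to HomeBase.
; Capsule overlap flags the player in range until Box1 exit, and Tick-driven DealDamage kills the player after a delay without rechecking range.
; FirstPersonProjectile capsule hits reduce the pawn's Health, destroying it at zero.
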(event OnComponentBeginOverlap(CapsuleComponent)
  (params (OverlappedComponent :type Primitive%20Component%20Object%20Reference) (OtherActor :type Actor%20Object%20Reference) (OtherComp :type Primitive%20Component%20Object%20Reference) (OtherBodyIndex :type Integer) (bFromSweep :type Boolean) (SweepResult :type Hit%20Result%20Structure%20%28by%20ref%29))
  (Utilities|FlowControl|Sequence
    (:then_0
      (Utilities|Casting|CastToFirstPersonProjectile OtherActor)
      (CallFunction|TakeDamage self))
    (:then_1
      (Utilities|Casting|CastToBP_Character OtherActor)
      (Variables|Default|Setenemyinrange true))))

(event OnComponentEndOverlap(Box2)
  (params (OverlappedComponent :type Primitive%20Component%20Object%20Reference) (OtherActor :type Actor%20Object%20Reference) (OtherComp :type Primitive%20Component%20Object%20Reference) (OtherBodyIndex :type Integer))
  (Utilities|Casting|CastToBP_Character OtherActor)
  (AI|AIMoveTo self (Variables|Default|GetHomeBase) 0 5.0 false))

(event OnComponentBeginOverlap(Box1)
  (params (OverlappedComponent :type Primitive%20Component%20Object%20Reference) (OtherActor :type Actor%20Object%20Reference) (OtherComp :type Primitive%20Component%20Object%20Reference) (OtherBodyIndex :type Integer) (bFromSweep :type Boolean) (SweepResult :type Hit%20Result%20Structure%20%28by%20ref%29)))

(event OnComponentBeginOverlap(Box2)
  (params (OverlappedComponent :type Primitive%20Component%20Object%20Reference) (OtherActor :type Actor%20Object%20Reference) (OtherComp :type Primitive%20Component%20Object%20Reference) (OtherBodyIndex :type Integer) (bFromSweep :type Boolean) (SweepResult :type Hit%20Result%20Structure%20%28by%20ref%29))
  (bind _asbp_character (Utilities|Casting|CastToBP_Character OtherActor))
  (AI|AIMoveTo self "0.000000,0.000000,0.000000" _asbp_character 5.0 false))

(event OnComponentEndOverlap(Box1)
  (params (OverlappedComponent :type Primitive%20Component%20Object%20Reference) (OtherActor :type Actor%20Object%20Reference) (OtherComp :type Primitive%20Component%20Object%20Reference) (OtherBodyIndex :type Integer))
  (Utilities|Casting|CastToBP_Character OtherActor)
  (Variables|Default|Setenemyinrange false))

(event Custom|Death
  (if (<= (Variables|Default|GetHealth) 0)
    (Actor|DestroyActor self)))

(event Custom|deal%20damage
  (if (Variables|Default|Getenemyinrange)
    (bind _asbp_character (Utilities|Casting|CastToBP_Character (Game|Player|GetPlayerPawn 0)))
    (Utilities|FlowControl|Delay 3.0)
    (Variables|/Game/Ninja/Blueprints/Character/BP_Character.BP_Character_C|SetHealth _asbp_character 0.0)
    (Development|PrintString (Utilities|String|ToString(Integer) 0))
    (Default|Death _asbp_character)))

(event Custom|Take%20Damage
  (Development|PrintString (Utilities|String|ToString(Integer) (Variables|Default|GetHealth)))
  (Variables|Default|SetHealth (- (Variables|Default|GetHealth) 10))
  (CallFunction|Death self))

(event EventTick
  (params (DeltaSeconds :type Float%20%28single-precision%29))
  (CallFunction|DealDamage))

(fn ConstructionScript)