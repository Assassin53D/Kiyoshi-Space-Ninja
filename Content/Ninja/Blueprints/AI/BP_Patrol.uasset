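; Patrolling enemy AI that chases a seen BP_Character and only prints "die" on touching it.
; Patrol loops through up to ten points using nested AIMoveTo calls with random waits, resuming after each chase.
; Projectile overlaps freeze and deactivate it for four seconds unless IsInLightning, while a separate Stun event halts movement, then restarts Patrol.
; Tick colours its light green, red or blue for patrolling, chasing or inactive, and locks rotation while inactive.
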(event OnComponentBeginOverlap(Box)
  (params (OverlappedComponent :type Primitive%20Component%20Object%20Reference) (OtherActor :type Actor%20Object%20Reference) (OtherComp :type Primitive%20Component%20Object%20Reference) (OtherBodyIndex :type Integer) (bFromSweep :type Boolean) (SweepResult :type Hit%20Result%20Structure%20%28by%20ref%29))
  (bind _charactermovement (Variables|Character|GetCharacterMovement))
  (Utilities|Casting|CastToFirstPersonProjectile OtherActor)
  (if (not (Variables|Default|GetIsInLightning))
    (Variables|Default|SetIsActive false)
    (Variables|/Script/Engine.CharacterMovementComponent|SetMaxWalkSpeed _charactermovement 0.0)
    (Utilities|FlowControl|RetriggerableDelay 4.0)
    (Variables|/Script/Engine.CharacterMovementComponent|SetMaxWalkSpeed _charactermovement 6e+02)
    (Variables|Default|SetIsActive true)))

(event OnComponentHit(CapsuleComponent)
  (params (HitComponent :type Primitive%20Component%20Object%20Reference) (OtherActor :type Actor%20Object%20Reference) (OtherComp :type Primitive%20Component%20Object%20Reference) (NormalImpulse :type Vector :default "0, 0, 0") (Hit :type Hit%20Result%20Structure%20%28by%20ref%29))
  (Utilities|Casting|CastToBP_Character OtherActor)
  (if (Variables|Default|GetIsActive)
    (Development|PrintString "die")))

(event OnSeePawn(PawnSensing)
  (params (Pawn :type Pawn%20Object%20Reference))
  (if (Variables|Default|GetIsActive)
    (bind _asbp_character (Utilities|Casting|CastToBP_Character Pawn))
    (Variables|Default|SetIsPatroling false)
    (AI|AIMoveTo self "0.000000,0.000000,0.000000" _asbp_character 5.0 false
      (:OnSuccess
        _)
      (:OnFail
        _))
    (Utilities|FlowControl|Delay 0.5)
    (CallFunction|Patrol)
    (Variables|Default|SetIsPatroling true)))

(event Custom|LightColour
  (if (Variables|Default|GetIsActive)
    (Variables|/Script/Engine.CharacterMovementComponent|SetRotationRate (Variables|Character|GetCharacterMovement) "0,540.000000, 0")
    (if (Variables|Default|GetIsPatroling)
      (Rendering|Components|Light|SetLightColor (Variables|Default|GetPointLight) (Variables|Default|GetGreenLightColour) true)
      (else
        (Rendering|Components|Light|SetLightColor (Variables|Default|GetPointLight) (Variables|Default|GetRedLightColour) true)))
    (else
      (Rendering|Components|Light|SetLightColor (Variables|Default|GetPointLight) (Variables|Default|GetBlueLightColour) true)
      (Variables|/Script/Engine.CharacterMovementComponent|SetRotationRate (Variables|Character|GetCharacterMovement) "0, 0, 0"))))

(event Custom|Stun
  (bind _charactermovement (Variables|Character|GetCharacterMovement))
  (Variables|/Script/Engine.CharacterMovementComponent|SetMaxWalkSpeed _charactermovement 0.0)
  (Utilities|FlowControl|Delay 4.0)
  (Variables|/Script/Engine.CharacterMovementComponent|SetMaxWalkSpeed _charactermovement 6e+02)
  (CallFunction|Patrol)
  (Variables|Default|SetIsActive true))

(event Custom|Patrol
  (if (Variables|Default|GetIsActive)
    (AI|AIMoveTo self "0,0.000000, 0" (Variables|Default|GetPatrolPoint_0) 5e+01 false
      (:OnSuccess
        (if (and (>= (Variables|Default|GetAmountpatrolpoints) 2) (Variables|Default|GetIsActive))
          (Utilities|FlowControl|Delay (Math|Random|RandomFloatinRange (Variables|Default|GetDelay0) (Variables|Default|GetDelay1)))
          (AI|AIMoveTo self "0, 0, 0" (Variables|Default|GetPatrolPoint_1) 5e+01 false
            (:OnSuccess
              (if (and (>= (Variables|Default|GetAmountpatrolpoints) 3) (Variables|Default|GetIsActive))
                (Utilities|FlowControl|Delay (Math|Random|RandomFloatinRange (Variables|Default|GetDelay0) (Variables|Default|GetDelay1)))
                (AI|AIMoveTo self "0, 0, 0" (Variables|Default|GetPatrolPoint_2) 5e+01 false
                  (:OnSuccess
                    (if (and (>= (Variables|Default|GetAmountpatrolpoints) 4) (Variables|Default|GetIsActive))
                      (Utilities|FlowControl|Delay (Math|Random|RandomFloatinRange (Variables|Default|GetDelay0) (Variables|Default|GetDelay1)))
                      (AI|AIMoveTo self "0, 0, 0" (Variables|Default|GetPatrolPoint_3) 5e+01 false
                        (:OnSuccess
                          (if (and (>= (Variables|Default|GetAmountpatrolpoints) 5) (Variables|Default|GetIsActive))
                            (Utilities|FlowControl|Delay (Math|Random|RandomFloatinRange (Variables|Default|GetDelay0) (Variables|Default|GetDelay1)))
                            (AI|AIMoveTo self "0, 0, 0" (Variables|Default|GetPatrolPoint_4) 5e+01 false
                              (:OnSuccess
                                (if (and (>= (Variables|Default|GetAmountpatrolpoints) 6) (Variables|Default|GetIsActive))
                                  (Utilities|FlowControl|Delay (Math|Random|RandomFloatinRange (Variables|Default|GetDelay0) (Variables|Default|GetDelay1)))
                                  (AI|AIMoveTo self "0, 0, 0" (Variables|Default|GetPatrolPoint_5) 5e+01 false
                                    (:OnSuccess
                                      (if (and (>= (Variables|Default|GetAmountpatrolpoints) 7) (Variables|Default|GetIsActive))
                                        (Utilities|FlowControl|Delay (Math|Random|RandomFloatinRange (Variables|Default|GetDelay0) (Variables|Default|GetDelay1)))
                                        (AI|AIMoveTo self "0, 0, 0" (Variables|Default|GetPatrolPoint_6) 5e+01 false
                                          (:OnSuccess
                                            (if (and (>= (Variables|Default|GetAmountpatrolpoints) 8) (Variables|Default|GetIsActive))
                                              (Utilities|FlowControl|Delay (Math|Random|RandomFloatinRange (Variables|Default|GetDelay0) (Variables|Default|GetDelay1)))
                                              (AI|AIMoveTo self "0, 0, 0" (Variables|Default|GetPatrolPoint_7) 5e+01 false
                                                (:OnSuccess
                                                  (if (and (>= (Variables|Default|GetAmountpatrolpoints) 9) (Variables|Default|GetIsActive))
                                                    (Utilities|FlowControl|Delay (Math|Random|RandomFloatinRange (Variables|Default|GetDelay0) (Variables|Default|GetDelay1)))
                                                    (AI|AIMoveTo self "0, 0, 0" (Variables|Default|GetPatrolPoint_8) 5e+01 false
                                                      (:OnSuccess
                                                        (if (and (>= (Variables|Default|GetAmountpatrolpoints) 10) (Variables|Default|GetIsActive))
                                                          (Utilities|FlowControl|Delay (Math|Random|RandomFloatinRange (Variables|Default|GetDelay0) (Variables|Default|GetDelay1)))
                                                          (AI|AIMoveTo self "0, 0,0.000000" (Variables|Default|GetPatrolPoint_9) 5e+01 false
                                                            (:OnSuccess
                                                              _)))))))))))))))))))))))))))
        (Utilities|FlowControl|Delay (Math|Random|RandomFloatinRange (Variables|Default|GetDelay0) (Variables|Default|GetDelay1)))
        (CallFunction|Patrol)))))

(event EventTick
  (params (DeltaSeconds :type Float%20%28single-precision%29))
  (CallFunction|LightColour))

(event EventBeginPlay
  (CallFunction|Patrol))

(fn ConstructionScript)