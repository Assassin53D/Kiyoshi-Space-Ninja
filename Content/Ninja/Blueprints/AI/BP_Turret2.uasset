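; BP_Turret2 is an AI turret that detects the player through a collision overlap and fires projectiles at them.
; Tick turns the barrel toward the found player and calls SpawnProjectile, rate-limited by a game-time check, unless the player is invisible.
; Light colour and audio reflect idle, targeting or stunned states; StuntImer clears a stun after a delay.
; IsActive gates new detection and light intensity, but not an ongoing attack.
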(event OnComponentBeginOverlap(Collision)
  (params (OverlappedComponent :type Primitive%20Component%20Object%20Reference) (OtherActor :type Actor%20Object%20Reference) (OtherComp :type Primitive%20Component%20Object%20Reference) (OtherBodyIndex :type Integer) (bFromSweep :type Boolean) (SweepResult :type Hit%20Result%20Structure%20%28by%20ref%29))
  (if (Variables|Default|GetIsActive)
    (if (not (Variables|Default|GetPlayerFound))
      (bind _asbp_character (Utilities|Casting|CastToBP_Character OtherActor))
      (Variables|Default|SetPlayerFound true))))

(event OnComponentEndOverlap(Collision)
  (params (OverlappedComponent :type Primitive%20Component%20Object%20Reference) (OtherActor :type Actor%20Object%20Reference) (OtherComp :type Primitive%20Component%20Object%20Reference) (OtherBodyIndex :type Integer))
  (Utilities|Casting|CastToBP_Character OtherActor)
  (Variables|Default|SetPlayerFound false))

(event Custom|Shoot%20Player
  (bind _barrelhead (Variables|Default|GetBarrelHead))
  (bind _asbp_character (Utilities|Casting|CastToBP_Character (Game|GetPlayerCharacter 0)))
  (if (not (Variables|/Game/Ninja/Blueprints/Character/BP_Character.BP_Character_C|GetIsInvisible _asbp_character))
    (if (Variables|Default|Getstunned)
      (Rendering|Components|Light|SetLightColor (Variables|Default|GetPointLight) (Variables|Default|GetBlueColour) true)
      (Components|Activation|Activate (Variables|Default|GetParticleSystem) false)
      (Utilities|FlowControl|DoOnce false :!label _label
        (:Completed
          (Audio|PlaySoundatLocation "/Game/Ninja/Audio/SFX_AIDisable_002_Cue.SFX_AIDisable_002_Cue" (Transformation|GetWorldLocation (Variables|Default|GetBase)))
          (Components|Activation|Deactivate (Variables|Default|GetAudio_Idle))))
      (else
        (Utilities|FlowControl|Sequence
          (:then_0
            (goto _label Reset))
          (:then_1
            (Components|Activation|Deactivate (Variables|Default|GetParticleSystem))
            (if (Variables|Default|GetPlayerFound)
              (Rendering|Components|Light|SetLightColor (Variables|Default|GetPointLight) (Variables|Default|GetRedColour) true)
              (Components|Activation|Deactivate (Variables|Default|GetAudio_Idle))
              (Transformation|SetWorldRotation (Variables|Default|GetBarrelHead) (Math|Interpolation|RInterpTo (Transformation|GetWorldRotation _barrelhead) (Math|Rotator|FindLookatRotation (Transformation|GetWorldLocation _barrelhead) (Transformation|GetWorldLocation (Variables|/Game/Ninja/Blueprints/Character/BP_Character.BP_Character_C|GetInteractionSpawn (stale OnComponentBeginOverlap(Collision) _asbp_character)))) 1.0 (Variables|Default|GetTurretRotationSpeed)) false false)
              (CallFunction|SpawnProjectile)
              (else
                (Rendering|Components|Light|SetLightColor (Variables|Default|GetPointLight) (Variables|Default|GetGreenColour) true)
                (Components|Activation|Activate (Variables|Default|GetAudio_Idle) false)))))))))

(event Custom|Stun%20tImer
  (Utilities|FlowControl|Delay 5.0)
  (Variables|Default|Setstunned false))

(event Custom|ActiveColour
  (bind _pointlight (Variables|Default|GetPointLight))
  (if (Variables|Default|GetIsActive)
    (Rendering|Components|Light|SetIntensity _pointlight 5e+03)
    (else
      (Rendering|Components|Light|SetIntensity _pointlight 0.0))))

(event EventBeginPlay
  (Components|Activation|Activate (Variables|Default|GetAudio_Idle) false))

(event EventTick
  (params (DeltaSeconds :type Float%20%28single-precision%29))
  (CallFunction|ShootPlayer)
  (CallFunction|ActiveColour))

(fn ConstructionScript)

(fn SpawnProjectile
  (bind _returnvalue (Utilities|Time|GetGameTimeinSeconds))
  (if (> _returnvalue (Variables|Default|GetGameTimeShoot))
    (Variables|Default|SetGameTimeShoot (+ _returnvalue (Variables|Default|GetShootDelay)))
    (Audio|PlaySoundatLocation "/Game/Ninja/Audio/SFX_LazerBig_003_Cue.SFX_LazerBig_003_Cue" (Transformation|GetWorldLocation (Variables|Default|GetBarrel)))
    (Game|SpawnActorfromClass "/Game/Ninja/Blueprints/AI/BP_TurretProjectile.BP_TurretProjectile_C" (Transformation|GetWorldTransform (Variables|Default|GetProjectileSpawn)) "Undefined" 0 0)))