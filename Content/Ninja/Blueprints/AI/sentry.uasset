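; Sentry AI actor that loses health when hit by first-person projectiles and destroys itself when health runs out.
; A Box overlap with a FirstPersonProjectile calls TakeDamage, which prints Health, subtracts a fixed amount, then runs the Death check.
; Player-character overlaps on both boxes only perform casts, and the PawnSensing see-pawn event is empty, so no detection behavior is implemented.
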(event OnComponentBeginOverlap(Box1)
  (params (OverlappedComponent :type Primitive%20Component%20Object%20Reference) (OtherActor :type Actor%20Object%20Reference) (OtherComp :type Primitive%20Component%20Object%20Reference) (OtherBodyIndex :type Integer) (bFromSweep :type Boolean) (SweepResult :type Hit%20Result%20Structure%20%28by%20ref%29))
  (Utilities|Casting|CastToFirstPersonCharacter OtherActor))

(event OnComponentBeginOverlap(Box)
  (params (OverlappedComponent :type Primitive%20Component%20Object%20Reference) (OtherActor :type Actor%20Object%20Reference) (OtherComp :type Primitive%20Component%20Object%20Reference) (OtherBodyIndex :type Integer) (bFromSweep :type Boolean) (SweepResult :type Hit%20Result%20Structure%20%28by%20ref%29))
  (Utilities|FlowControl|Sequence
    (:then_0
      (Utilities|Casting|CastToFirstPersonProjectile OtherActor)
      (CallFunction|TakeDamage self))
    (:then_1
      (Utilities|Casting|CastToFirstPersonCharacter OtherActor))))

(event OnComponentEndOverlap(Box1)
  (params (OverlappedComponent :type Primitive%20Component%20Object%20Reference) (OtherActor :type Actor%20Object%20Reference) (OtherComp :type Primitive%20Component%20Object%20Reference) (OtherBodyIndex :type Integer))
  (Utilities|Casting|CastToFirstPersonCharacter OtherActor))

(event OnSeePawn(PawnSensing)
  (params (Pawn :type Pawn%20Object%20Reference)))

(event Custom|Death
  (if (<= (Variables|Default|GetHealth) 0)
    (Actor|DestroyActor self)))

(event Custom|Take%20Damage
  (Development|PrintString (Utilities|String|ToString(Integer) (Variables|Default|GetHealth)))
  (Variables|Default|SetHealth (- (Variables|Default|GetHealth) 10))
  (CallFunction|Death self))

(fn ConstructionScript)