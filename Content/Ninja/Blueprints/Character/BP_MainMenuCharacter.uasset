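; Main menu character that spawns the menu widget on BeginPlay, shows the mouse cursor and drives button hover sounds.
; Each Tick, HoverButtons polls the widget's CurButton index to switch between the Play and Quit hover sound components.
; Paired DoOnce gates reset each other so a sound activates once per hover, and any other index silences both and rearms the gates.
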(event Custom|HoverButtons
  (bind _mainmenuref (Variables|Default|GetMainMenuRef))
  (if (== (Variables|/Game/Ninja/UI/MainMenuWidget.MainMenuWidget_C|GetCurButton _mainmenuref) 0)
    (Utilities|FlowControl|DoOnce false :!label _label
      (:Completed
        (Components|Activation|Activate (Variables|Default|GetPlayOverSound) false)
        (Components|Activation|Deactivate (Variables|Default|GetQuitHoverSound))
        (goto _label_2 Reset)))
    (elif (== (Variables|/Game/Ninja/UI/MainMenuWidget.MainMenuWidget_C|GetCurButton _mainmenuref) 1)
      (Utilities|FlowControl|DoOnce false :!label _label_2
        (:Completed
          (Components|Activation|Activate (Variables|Default|GetQuitHoverSound) false)
          (Components|Activation|Deactivate (Variables|Default|GetPlayOverSound))
          (goto _label Reset)))
      (else
        (Components|Activation|Deactivate (Variables|Default|GetQuitHoverSound))
        (Components|Activation|Deactivate (Variables|Default|GetPlayOverSound))
        (Utilities|FlowControl|Sequence
          (:then_0
            (goto _label_2 Reset))
          (:then_1
            (goto _label Reset)))))))

(event EventBeginPlay
  (bind _returnvalue (UserInterface|CreateWidget "/Game/Ninja/UI/MainMenuWidget.MainMenuWidget_C"))
  (bind _output_get (Variables|Default|SetMainMenuRef _returnvalue))
  (UserInterface|Viewport|AddtoViewport _output_get 0)
  (Variables|/Script/Engine.PlayerController|SetbShowMouseCursor (Game|GetPlayerController 0) true))

(event Collision|EventActorBeginOverlap
  (params (OtherActor :type Actor%20Object%20Reference)))

(event EventTick
  (params (DeltaSeconds :type Float%20%28single-precision%29))
  (CallFunction|HoverButtons))

(fn ConstructionScript)