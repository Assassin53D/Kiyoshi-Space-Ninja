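; Hologram wall trap that vanishes when a BP_Character or FirstPersonProjectile touches it, revealing it as an illusion.
; The box overlap plays a sound, hides the cube for a few seconds, then restores it with another sound.
; Every tick, MaterialChange checks the player's IsInvisible flag: while invisible, the point light shows and an intact wall switches from its basic material to a laser one.
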(event OnComponentBeginOverlap(Box)
  (params (OverlappedComponent :type Primitive%20Component%20Object%20Reference) (OtherActor :type Actor%20Object%20Reference) (OtherComp :type Primitive%20Component%20Object%20Reference) (OtherBodyIndex :type Integer) (bFromSweep :type Boolean) (SweepResult :type Hit%20Result%20Structure%20%28by%20ref%29))
  (Utilities|FlowControl|Sequence
    (:then_0
      (Utilities|Casting|CastToBP_Character OtherActor))
    (:then_1
      (Utilities|Casting|CastToFirstPersonProjectile OtherActor)))
  (Audio|PlaySoundatLocation 0 (Transformation|GetActorLocation)) ; Play firing sound
  (Variables|Default|SetIsAlive false)
  (Rendering|SetVisibility (Variables|Default|GetCube) false false)
  (Utilities|FlowControl|Delay 3.0)
  (Rendering|SetVisibility (Variables|Default|GetCube) true false)
  (Variables|Default|SetIsAlive true)
  (Audio|PlaySoundatLocation 0 (Transformation|GetActorLocation)) ; Play firing sound
)

(event Custom|MaterialChange
  (bind _cube (Variables|Default|GetCube))
  (bind _pointlight (Variables|Default|GetPointLight))
  (bind _asbp_character (Utilities|Casting|CastToBP_Character (Game|GetPlayerCharacter 0)))
  (if (Variables|Default|GetIsAlive)
    (if (Variables|/Game/Ninja/Blueprints/Character/BP_Character.BP_Character_C|GetIsInvisible _asbp_character)
      (Rendering|Material|SetMaterial _cube 0 "/Game/Ninja/Blueprints/Traps/las3er.las3er")
      (Rendering|SetVisibility _pointlight true false)
      (else
        (Rendering|Material|SetMaterial _cube 0 "/Engine/BasicShapes/BasicShapeMaterial.BasicShapeMaterial")
        (Rendering|SetVisibility _pointlight false false)))
    (else
      (Rendering|SetVisibility (Variables|Default|GetCube) false false)
      (if (Variables|/Game/Ninja/Blueprints/Character/BP_Character.BP_Character_C|GetIsInvisible _asbp_character)
        (Rendering|SetVisibility (Variables|Default|GetPointLight) true false)))))

(event EventBeginPlay)

(event Collision|EventActorBeginOverlap
  (params (OtherActor :type Actor%20Object%20Reference)))

(event EventTick
  (params (DeltaSeconds :type Float%20%28single-precision%29))
  (CallFunction|MaterialChange))

(fn ConstructionScript)