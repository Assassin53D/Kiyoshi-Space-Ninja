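; Laser trap actor that instantly kills a BP_Character standing inside its box trigger.
; Box overlap events store the character and toggle an in-range flag.
; While the flag is set, Tick sets the character's Health to zero, prints a debug zero and calls Death every frame.
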(event OnComponentBeginOverlap(Box)
  (params (OverlappedComponent :type Primitive%20Component%20Object%20Reference) (OtherActor :type Actor%20Object%20Reference) (OtherComp :type Primitive%20Component%20Object%20Reference) (OtherBodyIndex :type Integer) (bFromSweep :type Boolean) (SweepResult :type Hit%20Result%20Structure%20%28by%20ref%29))
  (bind _asbp_character (Utilities|Casting|CastToBP_Character OtherActor))
  (Variables|Default|Setenemyinrange true))

(event OnComponentEndOverlap(Box)
  (params (OverlappedComponent :type Primitive%20Component%20Object%20Reference) (OtherActor :type Actor%20Object%20Reference) (OtherComp :type Primitive%20Component%20Object%20Reference) (OtherBodyIndex :type Integer))
  (Utilities|Casting|CastToBP_Character OtherActor)
  (Variables|Default|Setenemyinrange false))

(event EventTick
  (params (DeltaSeconds :type Float%20%28single-precision%29))
  (if (Variables|Default|Getenemyinrange)
    (Variables|/Game/Ninja/Blueprints/Character/BP_Character.BP_Character_C|SetHealth (stale OnComponentBeginOverlap(Box) _asbp_character) 0.0)
    (Development|PrintString (Utilities|String|ToString(Integer) 0))
    (Default|Death (stale OnComponentBeginOverlap(Box) _asbp_character))))

(fn ConstructionScript)