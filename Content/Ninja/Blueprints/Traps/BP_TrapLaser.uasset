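; BP_TrapLaser is a laser trap that instantly kills a BP_Character overlapping its box while active.
; The IsActive flag gates the kill, which zeroes Health and calls Death, and is checked only when an overlap begins.
; Tick calls Activation every frame to match particle visibility to that flag.
; The laser audio activates one second after BeginPlay, independent of IsActive.
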(event OnComponentBeginOverlap(Box)
  (params (OverlappedComponent :type Primitive%20Component%20Object%20Reference) (OtherActor :type Actor%20Object%20Reference) (OtherComp :type Primitive%20Component%20Object%20Reference) (OtherBodyIndex :type Integer) (bFromSweep :type Boolean) (SweepResult :type Hit%20Result%20Structure%20%28by%20ref%29))
  (bind _asbp_character (Utilities|Casting|CastToBP_Character OtherActor))
  (if (Variables|Default|GetIsActive)
    (Variables|/Game/Ninja/Blueprints/Character/BP_Character.BP_Character_C|SetHealth _asbp_character 0.0)
    (Default|Death _asbp_character)))

(event Custom|Activation
  (bind _particlesystem (Variables|Default|GetParticleSystem))
  (if (Variables|Default|GetIsActive)
    (Rendering|SetVisibility _particlesystem true false)
    (else
      (Rendering|SetVisibility _particlesystem false false))))

(event EventBeginPlay
  (Utilities|FlowControl|Delay 1.0)
  (Components|Activation|Activate (Variables|Default|GetAudio_Laser) false))

(event EventTick
  (params (DeltaSeconds :type Float%20%28single-precision%29))
  (CallFunction|Activation))

(fn ConstructionScript)