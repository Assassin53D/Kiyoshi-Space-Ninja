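; BP_CrippleBubble is a short-lived trap that changes the state of characters inside its bubble, presumably crippling them.
; On spawn it plays a sound at its location, then destroys itself after a fixed delay.
; Sphere overlap begin and end each set a different States value on the overlapping BP_Character and call its StateChange, which applies the effect.
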(event OnComponentEndOverlap(Sphere)
  (params (OverlappedComponent :type Primitive%20Component%20Object%20Reference) (OtherActor :type Actor%20Object%20Reference) (OtherComp :type Primitive%20Component%20Object%20Reference) (OtherBodyIndex :type Integer))
  (bind _asbp_character (Utilities|Casting|CastToBP_Character OtherActor))
  (Variables|/Game/Ninja/Blueprints/Character/BP_Character.BP_Character_C|SetStates _asbp_character "NewEnumerator1")
  (Default|StateChange _asbp_character))

(event OnComponentBeginOverlap(Sphere)
  (params (OverlappedComponent :type Primitive%20Component%20Object%20Reference) (OtherActor :type Actor%20Object%20Reference) (OtherComp :type Primitive%20Component%20Object%20Reference) (OtherBodyIndex :type Integer) (bFromSweep :type Boolean) (SweepResult :type Hit%20Result%20Structure%20%28by%20ref%29))
  (bind _asbp_character (Utilities|Casting|CastToBP_Character OtherActor))
  (Variables|/Game/Ninja/Blueprints/Character/BP_Character.BP_Character_C|SetStates _asbp_character "NewEnumerator0")
  (Default|StateChange _asbp_character))

(event EventBeginPlay
  (Audio|PlaySoundatLocation 0 (Transformation|GetActorLocation))
  (Utilities|FlowControl|Delay 7.0)
  (Actor|DestroyActor))

(event Collision|EventActorBeginOverlap
  (params (OtherActor :type Actor%20Object%20Reference)))

(event EventTick
  (params (DeltaSeconds :type Float%20%28single-precision%29)))

(fn ConstructionScript)