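; BP_TrapSpike is a trap that kills the player character and is revealed while the player is invisible.
; Each Tick, until destroyed, it swaps the cube's material and toggles a point light based on the player's IsInvisible flag.
; Box overlaps by the character or a FirstPersonProjectile set Destroyed and hide the cube.
; Box1 overlaps play a sound, zero the character's Health and call Death, regardless of Destroyed.
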(event OnComponentBeginOverlap(Box)
  (params (OverlappedComponent :type Primitive%20Component%20Object%20Reference) (OtherActor :type Actor%20Object%20Reference) (OtherComp :type Primitive%20Component%20Object%20Reference) (OtherBodyIndex :type Integer) (bFromSweep :type Boolean) (SweepResult :type Hit%20Result%20Structure%20%28by%20ref%29))
  (Utilities|FlowControl|Sequence
    (:then_0
      (Utilities|Casting|CastToBP_Character OtherActor))
    (:then_1
      (Utilities|Casting|CastToFirstPersonProjectile OtherActor)
      (Audio|PlaySoundatLocation 0 (Transformation|GetActorLocation)) ; Play firing sound
    ))
  (Variables|Default|SetDestroyed true)
  (Rendering|SetVisibility (Variables|Default|GetCube) false false))

(event OnComponentBeginOverlap(Box1)
  (params (OverlappedComponent :type Primitive%20Component%20Object%20Reference) (OtherActor :type Actor%20Object%20Reference) (OtherComp :type Primitive%20Component%20Object%20Reference) (OtherBodyIndex :type Integer) (bFromSweep :type Boolean) (SweepResult :type Hit%20Result%20Structure%20%28by%20ref%29))
  (bind _asbp_character (Utilities|Casting|CastToBP_Character OtherActor))
  (Audio|PlaySoundatLocation 0 (Transformation|GetActorLocation)) ; Play firing sound
  (Variables|/Game/Ninja/Blueprints/Character/BP_Character.BP_Character_C|SetHealth _asbp_character 0.0)
  (Default|Death _asbp_character))

(event Custom|MaterialChange
  (bind _cube (Variables|Default|GetCube))
  (bind _pointlight (Variables|Default|GetPointLight))
  (bind _asbp_character (Utilities|Casting|CastToBP_Character (Game|GetPlayerCharacter 0)))
  (if (not (Variables|Default|GetDestroyed))
    (if (Variables|/Game/Ninja/Blueprints/Character/BP_Character.BP_Character_C|GetIsInvisible _asbp_character)
      (Rendering|Material|SetMaterial _cube 0 "/Game/Ninja/Blueprints/Traps/las3er.las3er")
      (Rendering|SetVisibility _pointlight true false)
      (else
        (Rendering|Material|SetMaterial _cube 0 "/Engine/BasicShapes/BasicShapeMaterial.BasicShapeMaterial")
        (Rendering|SetVisibility _pointlight false false)))))

(event EventBeginPlay)

(event Collision|EventActorBeginOverlap
  (params (OtherActor :type Actor%20Object%20Reference)))

(event EventTick
  (params (DeltaSeconds :type Float%20%28single-precision%29))
  (CallFunction|MaterialChange))

(fn ConstructionScript)