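; Cripple trap actor that shows its mesh, steam and light only while the player character is invisible, checked every tick.
; A player entering its trigger while it is armed spawns a cripple bubble at the arrow, gated by a DoOnce that resets on overlaps while disarmed.
; A first-person projectile hit disarms it with a sound.
; Either event hides the mesh and starts a retriggerable timer that re-arms the trap.
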(event OnComponentBeginOverlap(Box)
  (params (OverlappedComponent :type Primitive%20Component%20Object%20Reference) (OtherActor :type Actor%20Object%20Reference) (OtherComp :type Primitive%20Component%20Object%20Reference) (OtherBodyIndex :type Integer) (bFromSweep :type Boolean) (SweepResult :type Hit%20Result%20Structure%20%28by%20ref%29))
  (bind _audio (Variables|Default|GetAudio))
  (Utilities|Casting|CastToFirstPersonProjectile OtherActor)
  (Variables|Default|SetIsAlive false)
  (Audio|Components|Audio|Play _audio 0.0)
  (Transformation|SetWorldLocation _audio (Transformation|GetActorLocation) false false)
  (CallFunction|ActivationTimer))

(event OnComponentBeginOverlap(Box1)
  (params (OverlappedComponent :type Primitive%20Component%20Object%20Reference) (OtherActor :type Actor%20Object%20Reference) (OtherComp :type Primitive%20Component%20Object%20Reference) (OtherBodyIndex :type Integer) (bFromSweep :type Boolean) (SweepResult :type Hit%20Result%20Structure%20%28by%20ref%29))
  (Utilities|Casting|CastToBP_Character OtherActor)
  (if (Variables|Default|GetIsAlive)
    (Utilities|FlowControl|DoOnce false :!label _label
      (:Completed
        (Variables|Default|SetIsAlive false)
        (Variables|Default|SetIsTrapOn true)
        (Game|SpawnActorfromClass "/Game/Ninja/Blueprints/Traps/BP_CrippleBubble.BP_CrippleBubble_C" (Transformation|GetWorldTransform (Variables|Default|GetArrow)) "Undefined" 0 0)
        (Utilities|FlowControl|Delay 0.2)
        (Audio|Components|Audio|Stop (Variables|Default|GetAudio))
        (Variables|Default|SetIsTrapOn false)
        (CallFunction|ActivationTimer)))
    (else
      (goto _label Reset))))

(event Custom|Activated?
  (bind _cube (Variables|Default|GetCube))
  (if (Variables|Default|GetIsAlive)
    (bind _asbp_character (Utilities|Casting|CastToBP_Character (Game|GetPlayerCharacter 0)))
    (if (Variables|/Game/Ninja/Blueprints/Character/BP_Character.BP_Character_C|GetIsInvisible _asbp_character)
      (Rendering|SetVisibility _cube true false)
      (else
        (Rendering|SetVisibility _cube false false)))
    (else
      (Rendering|SetVisibility (Variables|Default|GetCube) false false)
      (if (Variables|/Game/Ninja/Blueprints/Character/BP_Character.BP_Character_C|GetIsInvisible _asbp_character)
        (Rendering|SetVisibility (Variables|Default|GetP_Steam_Lit2) true false)))))

(event Custom|ActivationTimer
  (Utilities|FlowControl|RetriggerableDelay 5.0)
  (Variables|Default|SetIsAlive true))

(event EventBeginPlay
  (Audio|Components|Audio|SetSound (Variables|Default|GetAudio) "/Game/Ninja/Audio/SFX_CrippledTrap_Trigger_003.SFX_CrippledTrap_Trigger_003"))

(event Collision|EventActorBeginOverlap
  (params (OtherActor :type Actor%20Object%20Reference)))

(event EventTick
  (params (DeltaSeconds :type Float%20%28single-precision%29))
  (CallFunction|Activated?))

(fn ConstructionScript)